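; Player character Blueprint that ties death, respawning and UI input to the game mode and HUD.
; On BeginPlay it stores its transform in BP_GameMode as the respawn point.
; HealthComponent death destroys the current weapon and the character, and the Destroyed event asks the game mode for a delayed respawn.
; M shows the main menu through BP_HUD, while F simulates a left click through the WidgetInteraction component.
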(event `self.ReceiveBeginPlay`
  (bind _asbp_game_mode (cast `/Game/JoyWay/Blueprints/BP_GameMode` (`GameplayStatics.GetGameMode`)))
  (set `/Game/JoyWay/Blueprints/BP_GameMode.Respawn Transform` (`self.GetTransform`) _asbp_game_mode))

(event `Key|M`
  (params (Key :type "Key Structure"))
  (:`Pressed`
    (bind _asbp_hud (cast `/Game/JoyWay/Blueprints/BP_HUD` (`PlayerController.GetHUD` (`GameplayStatics.GetPlayerController` 0))))
    (`MyHUD.ShowWidget` _asbp_hud "MainMenu" 0)))

(event `self.HealthComponent.OnDie`
  (bind _currentweapon (`self.CurrentWeapon`)
    (:`then`
      (`self.K2_DestroyActor` _currentweapon))
    (:`else`
      _))
  (`self.K2_DestroyActor`))

(event `Key|F`
  (params (Key :type "Key Structure"))
  (bind _widgetinteraction (`self.WidgetInteraction`))
  (:`Pressed`
    (`WidgetInteractionComponent.PressPointerKey` _widgetinteraction "LeftMouseButton")
    (`WidgetInteractionComponent.ReleasePointerKey` _widgetinteraction "LeftMouseButton")))

(event `self.ReceiveDestroyed`
  (bind _asbp_game_mode (cast `/Game/JoyWay/Blueprints/BP_GameMode` (`GameplayStatics.GetGameMode`)))
  (`/Game/JoyWay/Blueprints/BP_GameMode.RespawnPlayer` _asbp_game_mode 1.0 self))

(fn `UserConstructionScript`)