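; Game mode that saves and restores the player's state and handles respawning.
; SaveGame writes a fresh slot, reloads it, then SavePawn fills in inventory, health and any equipped weapon with ammo.
; BeginPlay restores that state and deletes the slot afterwards, but a failed weapon cast stops it before health and deletion.
; RespawnPlayer waits, spawns the character's class at RespawnTransform, possesses it and shows the in-game HUD.
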(event `self.ReceiveBeginPlay`
  (bind _returnvalue (`GameplayStatics.DoesSaveGameExist` (`self.SaveName`)))
  (if _returnvalue
    (bind _returnvalue_2 (`GameplayStatics.LoadGameFromSlot` (`self.SaveName`)))
    (bind _asbp_save_game (cast `/Game/JoyWay/Blueprints/BP_SaveGame` _returnvalue_2))
    (bind _asbp_player_character (cast `/Game/JoyWay/Blueprints/BP_PlayerCharacter` (`GameplayStatics.GetPlayerCharacter` 0)))
    (set `InventoryComponent.Items` (`/Game/JoyWay/Blueprints/BP_SaveGame.Items` _asbp_save_game) (`JoyWayCharacter.InventoryComponent` _asbp_player_character))
    (bind _weaponinfo (`/Game/JoyWay/Blueprints/BP_SaveGame.WeaponInfo` _asbp_save_game))
    (set `JoyWayCharacter.WeaponInfo` _weaponinfo _asbp_player_character)
    (bind _asweapon_base (castclass `WeaponBase` (`.Container` (break `InventoryItemInfo` _weaponinfo))))
    (`JoyWayCharacter.EquipWeapon` _asbp_player_character _asweapon_base)
    (set `WeaponBase.CurrentAmmo` (`/Game/JoyWay/Blueprints/BP_SaveGame.CurrentAmmo` _asbp_save_game) (`JoyWayCharacter.CurrentWeapon` _asbp_player_character))
    (set `HealthComponent.CurrentHealth` (`/Game/JoyWay/Blueprints/BP_SaveGame.CurrentHealth` _asbp_save_game) (`JoyWayCharacter.HealthComponent` _asbp_player_character))
    (`GameplayStatics.DeleteGameInSlot` (`self.SaveName`))))

(event `SaveGame`
  (bind _returnvalue (`GameplayStatics.CreateSaveGameObject` "/Game/JoyWay/Blueprints/BP_SaveGame.BP_SaveGame_C"))
  (`GameplayStatics.SaveGameToSlot` _returnvalue (`self.SaveName`))
  (bind _asbp_player_character (cast `/Game/JoyWay/Blueprints/BP_PlayerCharacter` (`GameplayStatics.GetPlayerCharacter` 0)))
  (bind _returnvalue_2 (`GameplayStatics.LoadGameFromSlot` (`self.SaveName`)))
  (bind _asbp_save_game (cast `/Game/JoyWay/Blueprints/BP_SaveGame` _returnvalue_2))
  (`self.SavePawn` _asbp_player_character _asbp_save_game))

(event `RespawnPlayer`
  (params (DelayDuration :type "Float (double-precision)") (Character :type "/Game/JoyWay/Blueprints/BP_PlayerCharacter Object Reference"))
  (bind _returnvalue (`GameplayStatics.GetPlayerController` 0))
  (`KismetSystemLibrary.Delay` DelayDuration)
  (bind _returnvalue_2 (`|SpawnActorFromClass` (`GameplayStatics.GetObjectClass` Character) (`self.Respawn Transform`) "Undefined" "OverrideRootScale" null null))
  (`Controller.Possess` _returnvalue _returnvalue_2)
  (bind _asbp_hud (cast `/Game/JoyWay/Blueprints/BP_HUD` (`PlayerController.GetHUD` _returnvalue)))
  (`MyHUD.ShowWidget` _asbp_hud "InGame" 0))

(fn `SavePawn`
  (params (PlayerRef :type "/Game/JoyWay/Blueprints/BP_PlayerCharacter Object Reference") (SaveGame :type "/Game/JoyWay/Blueprints/BP_SaveGame Object Reference"))
  (bind _currentweapon (`JoyWayCharacter.CurrentWeapon` PlayerRef))
  (set `/Game/JoyWay/Blueprints/BP_SaveGame.Items` (`InventoryComponent.Items` (`JoyWayCharacter.InventoryComponent` PlayerRef)) SaveGame)
  (set `/Game/JoyWay/Blueprints/BP_SaveGame.CurrentHealth` (`HealthComponent.CurrentHealth` (`JoyWayCharacter.HealthComponent` PlayerRef)) SaveGame)
  (`/Engine/EditorBlueprintResources/StandardMacros.IsValid` _currentweapon
    (:`Is Valid`
      (set `/Game/JoyWay/Blueprints/BP_SaveGame.WeaponInfo` (`JoyWayCharacter.WeaponInfo` PlayerRef) SaveGame)
      (set `/Game/JoyWay/Blueprints/BP_SaveGame.CurrentAmmo` (`WeaponBase.CurrentAmmo` _currentweapon) SaveGame))
    (:`Is Not Valid`
      _))
  (`GameplayStatics.SaveGameToSlot` SaveGame (`self.SaveName`)))

(fn `UserConstructionScript`)